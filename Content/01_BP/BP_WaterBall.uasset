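; BP_WaterBall is a water ball actor that can feed its water quantity into the active floor's water timeline when it collides.
; All logic runs on the server through its sphere's overlap and hit events.
; Overlapping a BP_Wall in one of two states marks it safe, while other states trigger the water and destroy it.
; On a hit it is destroyed, triggering the water through GM_Gameplay unless marked safe.
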(event OnComponentBeginOverlap(Sphere)
  (params (OverlappedComponent :type Primitive%20Component%20Object%20Reference) (OtherActor :type Actor%20Object%20Reference) (OtherComp :type Primitive%20Component%20Object%20Reference) (OtherBodyIndex :type Integer) (bFromSweep :type Boolean) (SweepResult :type Hit%20Result%20Structure%20%28by%20ref%29))
  (if (Networking|IsServer)
    (bind _asbp_wall (Utilities|Casting|CastToBP_Wall OtherActor))
    (if (or (Utilities|Enum|Equal(Enum) (Variables|/Game/01_BP/Wall/BP_Wall.BP_Wall_C|GetState _asbp_wall) "NewEnumerator0") (Utilities|Enum|Equal(Enum) (Variables|/Game/01_BP/Wall/BP_Wall.BP_Wall_C|GetState _asbp_wall) "NewEnumerator3"))
      (Variables|Default|SetSafe true)
      (else
        (bind _asgm_gameplay (Utilities|Casting|CastToGM_Gameplay (Game|GetGameMode)))
        (Default|ESetWatterTimeline (Utilities|Array|Get(acopy) (Variables|/Game/01_BP/GM_Gameplay.GM_Gameplay_C|GetListeEtage _asgm_gameplay) (Variables|/Game/01_BP/GM_Gameplay.GM_Gameplay_C|GetActiveFloor _asgm_gameplay)) (Variables|Default|GetWaterQuantity))
        (Actor|DestroyActor)))))

(event OnComponentHit(Sphere)
  (params (HitComponent :type Primitive%20Component%20Object%20Reference) (OtherActor :type Actor%20Object%20Reference) (OtherComp :type Primitive%20Component%20Object%20Reference) (NormalImpulse :type Vector :default "0, 0, 0") (Hit :type Hit%20Result%20Structure%20%28by%20ref%29))
  (if (Networking|IsServer)
    (if (Variables|Default|GetSafe)
      (Actor|DestroyActor)
      (else
        (bind _asgm_gameplay (Utilities|Casting|CastToGM_Gameplay (Game|GetGameMode)))
        (Default|ESetWatterTimeline (Utilities|Array|Get(acopy) (Variables|/Game/01_BP/GM_Gameplay.GM_Gameplay_C|GetListeEtage _asgm_gameplay) (Variables|/Game/01_BP/GM_Gameplay.GM_Gameplay_C|GetActiveFloor _asgm_gameplay)) (Variables|Default|GetWaterQuantity))
        (Actor|DestroyActor)))))

(fn ConstructionScript)