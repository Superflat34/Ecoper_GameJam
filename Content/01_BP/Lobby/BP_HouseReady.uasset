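; Lobby ready zone that starts the game once every player stands inside its box.
; The server counts overlaps against the GameMode's player list, runs a three-second countdown, then calls the GameMode's start function once, resetting if the count no longer matches.
; A widget that turns toward the camera shows the ready count or countdown, updated through a text event.
; A separate event triggers the loading screen.
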(event OnComponentBeginOverlap(Box)
  (params (OverlappedComponent :type Primitive%20Component%20Object%20Reference) (OtherActor :type Actor%20Object%20Reference) (OtherComp :type Primitive%20Component%20Object%20Reference) (OtherBodyIndex :type Integer) (bFromSweep :type Boolean) (SweepResult :type Hit%20Result%20Structure%20%28by%20ref%29))
  (if (Networking|IsServer)
    (Math|Integer|IncrementInt (Variables|Default|GetNBPlayerReady))))

(event OnComponentEndOverlap(Box)
  (params (OverlappedComponent :type Primitive%20Component%20Object%20Reference) (OtherActor :type Actor%20Object%20Reference) (OtherComp :type Primitive%20Component%20Object%20Reference) (OtherBodyIndex :type Integer))
  (if (Networking|IsServer)
    (Math|Integer|DecrementInt (Variables|Default|GetNBPlayerReady))))

(event Custom|E_LoadScreen
  (CallFunction|FLoadingScreen))

(event Custom|E_SetTextClient
  (params (Text :type Text))
  (Default|ESetText (Variables|Default|GetTextWidget) Text 5e+01))

(event EventBeginPlay
  (bind _aswbp_text (Utilities|Casting|CastToWBP_Text (UserInterface|GetUserWidgetObject (Variables|Default|GetWidget))))
  (Variables|Default|SetTextWidget _aswbp_text)
  (if (Networking|IsServer)
    (bind _asgm_gameplay (Utilities|Casting|CastToGM_Gameplay (Game|GetGameMode)))
    (Variables|Default|SetGM _asgm_gameplay)))

(event EventTick
  (params (DeltaSeconds :type Float%20%28single-precision%29))
  (bind _gm (Variables|Default|GetGM))
  (bind _nbplayerready (Variables|Default|GetNBPlayerReady))
  (bind _listplayer (Variables|/Game/01_BP/GM_Gameplay.GM_Gameplay_C|GetListPlayer _gm))
  (bind _returnvalue (Utilities|Array|Length _listplayer))
  (Variables|Default|SetDeltaTime DeltaSeconds)
  (CallFunction|FUiRotateTowardCam)
  (if (Networking|IsServer)
    (if (== _nbplayerready _returnvalue)
      (CallFunction|FCountBeforeStratGame)
      (if (>= (+ (Variables|Default|GetTimer) (Variables|Default|GetDeltaTime)) 3.0)
        (Utilities|FlowControl|DoOnce false :!label _label
          (:Completed
            (Default|FStartGame (Variables|Default|GetGM)))))
      (else
        (Variables|Default|SetTimer 0.0)
        (CallFunction|ESetTextClient (Utilities|Text|ToText(String) (Utilities|String|Append "Player Ready : " (Utilities|String|ToString(Integer) _nbplayerready) " / " (Utilities|String|ToString(Integer) _returnvalue))))
        (goto _label Reset)))))

(fn ConstructionScript)

(fn FCountBeforeStratGame
  (bind _output_get (Variables|Default|SetTimer (+ (Variables|Default|GetTimer) (Variables|Default|GetDeltaTime))))
  (Development|PrintString (Utilities|String|Append "Time Before Strating : " (Utilities|String|ToString(Float) _output_get)) true true "(R=0.000000,G=0.660000,B=1.000000,A=1.000000)" 0.0)
  (CallFunction|ESetTextClient (Utilities|Text|ToText(String) (Utilities|String|Append "Starting in " (Utilities|String|ToString(Integer) (Class|KismetMathLibrary|ToInt64(Float) (- 3.0 (+ (Math|Float|Clamp(Float) (Variables|Default|GetTimer) 0.0 3.0) -1.0))))))))

(fn FUiRotateTowardCam
  (bind _returnvalue (Game|GetPlayerCameraManager 0))
  (bind _widget (Variables|Default|GetWidget))
  (Utilities|IsValid _returnvalue
    (:Is%20Valid
      (Utilities|IsValid _widget
        (:Is%20Valid
          (Transformation|SetWorldRotation _widget (Math|Rotator|FindLookatRotation (Transformation|GetWorldLocation (Variables|Default|GetWidget)) (Transformation|GetActorLocation _returnvalue)) false false))))))