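; BP_Credit is a lobby actor that displays a floating "credit" label through a world widget.
; BeginPlay sets the WBP_Text label and adds a hidden WBP_Option widget to the viewport.
; Tick rotates the label toward the player camera.
; Box overlaps check for an active BP_Player but do nothing, as the logic toggling the option widget and mouse cursor is disconnected.
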(event OnComponentBeginOverlap(Box)
  (params (OverlappedComponent :type Primitive%20Component%20Object%20Reference) (OtherActor :type Actor%20Object%20Reference) (OtherComp :type Primitive%20Component%20Object%20Reference) (OtherBodyIndex :type Integer) (bFromSweep :type Boolean) (SweepResult :type Hit%20Result%20Structure%20%28by%20ref%29))
  (bind _asbp_player (Utilities|Casting|CastToBP_Player OtherActor))
  (if (Variables|/Game/01_BP/Player/BP_Player.BP_Player_C|GetActive _asbp_player)
    _))

(event OnComponentEndOverlap(Box)
  (params (OverlappedComponent :type Primitive%20Component%20Object%20Reference) (OtherActor :type Actor%20Object%20Reference) (OtherComp :type Primitive%20Component%20Object%20Reference) (OtherBodyIndex :type Integer))
  (bind _asbp_player (Utilities|Casting|CastToBP_Player OtherActor))
  (if (Variables|/Game/01_BP/Player/BP_Player.BP_Player_C|GetActive _asbp_player)
    _))

(event Custom|E_SetTextClient
  (params (Text :type Text))
  (Default|ESetText (Variables|Default|GetTextWidget) Text 5e+01))

(event EventTick
  (params (DeltaSeconds :type Float%20%28single-precision%29))
  (CallFunction|FUiRotateTowardCam))

(event EventBeginPlay
  (bind _aswbp_text (Utilities|Casting|CastToWBP_Text (UserInterface|GetUserWidgetObject (Variables|Default|GetWidget))))
  (Variables|Default|SetTextWidget _aswbp_text)
  (CallFunction|ESetTextClient "credit")
  (bind _returnvalue (UserInterface|CreateWidget "/Game/06_Widget/WBP_Option.WBP_Option_C"))
  (bind _output_get (Variables|Default|SetOptionWidget _returnvalue))
  (Utilities|IsValid _output_get
    (:Is%20Valid
      (Widget|SetVisibility _output_get "Hidden")
      (UserInterface|Viewport|AddtoViewport _output_get 10))))

(fn ConstructionScript)

(fn FUiRotateTowardCam
  (bind _returnvalue (Game|GetPlayerCameraManager 0))
  (bind _widget (Variables|Default|GetWidget))
  (Utilities|IsValid _returnvalue
    (:Is%20Valid
      (Utilities|IsValid _widget
        (:Is%20Valid
          (Transformation|SetWorldRotation _widget (Math|Rotator|FindLookatRotation (Transformation|GetWorldLocation (Variables|Default|GetWidget)) (Transformation|GetActorLocation _returnvalue)) false false))))))