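; BP_Camera is a player-following camera actor that becomes the local view target once the player is active.
; Each tick it sweeps SpringArmCol to the player's location and moves SpringArmCam likewise, with collision sweeps.
; While its Box overlaps something, SpringArmCam holds its Y and follows only X and Z, unless the player is beyond a distance threshold.
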(event OnComponentBeginOverlap(Box)
  (params (OverlappedComponent :type Primitive%20Component%20Object%20Reference) (OtherActor :type Actor%20Object%20Reference) (OtherComp :type Primitive%20Component%20Object%20Reference) (OtherBodyIndex :type Integer) (bFromSweep :type Boolean) (SweepResult :type Hit%20Result%20Structure%20%28by%20ref%29))
  (Variables|Default|SetLimited true))

(event OnComponentEndOverlap(Box)
  (params (OverlappedComponent :type Primitive%20Component%20Object%20Reference) (OtherActor :type Actor%20Object%20Reference) (OtherComp :type Primitive%20Component%20Object%20Reference) (OtherBodyIndex :type Integer))
  (Variables|Default|SetLimited false))

(event EventTick
  (params (DeltaSeconds :type Float%20%28single-precision%29))
  (bind _springarmcam (Variables|Default|GetSpringArmCam))
  (bind _player (Variables|Default|GetPlayer))
  (bind _returnvalue (Transformation|GetActorLocation _player))
  (Utilities|FlowControl|Sequence
    (:then_0
      (if (Variables|/Game/01_BP/Player/BP_Player.BP_Player_C|GetActive (Variables|Default|GetPlayer))
        (Utilities|FlowControl|DoOnce false
          (:Completed
            (Game|Player|SetViewTargetwithBlend (Pawn|GetLocalViewingPlayerController (Variables|Default|GetPlayer)) self 0.0 "VTBlend_Linear" 0.0 false)))))
    (:then_1
      (Transformation|SetWorldLocation (Variables|Default|GetSpringArmCol) (Transformation|GetActorLocation (Variables|Default|GetPlayer)) true false)
      (if (or (not (Variables|Default|GetLimited)) (> (Math|Vector|Distance(Vector) (Transformation|GetActorLocation (Variables|Default|GetPlayer)) (Transformation|GetWorldLocation (Variables|Default|GetSpringArmCam))) 1.25e+03))
        (Transformation|SetWorldLocation _springarmcam (Math|Vector|MakeVector (.x _returnvalue) (.y _returnvalue) (.z _returnvalue)) true false)
        (else
          (Transformation|SetWorldLocation _springarmcam (Math|Vector|MakeVector (.x _returnvalue) (.y (Transformation|GetWorldLocation (Variables|Default|GetSpringArmCam))) (.z _returnvalue)) true false))))))

(fn ConstructionScript)