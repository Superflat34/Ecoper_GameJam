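; Multiplayer game mode that runs a timed preparation phase, then the main round on floors with water levels and breakable walls.
; It spawns and tracks a pawn per joining player, and scatters interactables and movables at random spawn points from player-count maps.
; A Tick-driven timer switches phases, activates floor 3 and ends the round on timeout, teleporting players and resetting state.
; It also forwards input to player 0, handles ServerTravel and prints debug info.
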(event Custom|E_ActiveFloor
  (params (Floor :type Integer))
  (bind _listeetage (Variables|Default|GetListeEtage))
  (bind _output (Utilities|Array|Get(acopy) _listeetage Floor))
  (bind _door (Variables|/Game/01_BP/Wall/BP_Floor.BP_Floor_C|GetDoor _output))
  (Default|EActiveFloorClient _output true)
  (Utilities|IsValid _door
    (:Is%20Valid
      (Default|EChangeStateClient _door "NewEnumerator3" 4e+01))
    (:Is%20Not%20Valid
      _))
  (Variables|Default|SetActiveFloor Floor)
  (if (!= Floor 0)
    (for _array_element (Variables|Default|GetListPlayer)
      (Default|EMoveClient _array_element (+ (Transformation|GetActorLocation _output) "0.000000,0.000000,75.000000")))))

(event Custom|E_SetPlayerID
  (for (_array_element _array_index) (Variables|Default|GetListPlayer)
    (Default|ESetPlayerIdClient _array_element _array_index)))

(event Custom|E_FinishGame
  (params (WIn :type E_Win%20Enum :default "NewEnumerator0"))
  (Variables|Game|SetGameStart false)
  (Variables|Default|SetActiveFloor 0)
  (CallFunction|EDestroyAllInetractable)
  (Utilities|FlowControl|Sequence
    (:then_0
      (Variables|Game|SetTimerGame 0.0)
      (for _array_element (Variables|Default|GetListPlayer)
        (Default|EMoveClient _array_element "0.000000,0.000000,125.000000")
        (Default|EFinishGame _array_element WIn)
        (Default|EReset _array_element)))
    (:then_1
      (for _array_element_2 (Variables|Default|GetListeEtage)
        (Variables|/Game/01_BP/Wall/BP_Floor.BP_Floor_C|SetActive _array_element_2 false)
        (Variables|/Game/01_BP/Wall/BP_Floor.BP_Floor_C|SetWaterLevelPercent _array_element_2 0.0)
        (Variables|/Game/01_BP/Wall/BP_Floor.BP_Floor_C|SetTimerWallBreak _array_element_2 0.0)
        (Default|FResetAllWall _array_element_2)))))

(event Custom|E_DestroyAllInetractable
  (for _array_element (Variables|Interactable|GetListInteractable)
    (Utilities|IsValid _array_element
      (:Is%20Valid
        (Actor|DestroyActor _array_element))))
  (Utilities|Array|Clear (Variables|Interactable|GetListInteractable)))

(event Custom|E_SpawnInteractable
  (switch int (Utilities|Array|Length (Variables|Default|GetListPlayer))
    (:Default
      (bind _output_get (Variables|Interactable|SetMapInterUse (Variables|Interactable|GetMapInteractableP1) :!label _label)))
    (:1
      (goto _label))
    (:2
      (Variables|Interactable|SetMapInterUse (Variables|Interactable|GetMapInteractableP2)))
    (:3
      (Variables|Interactable|SetMapInterUse (Variables|Interactable|GetMapInteractableP3)))
    (:4
      (Variables|Interactable|SetMapInterUse (Variables|Interactable|GetMapInteractableP4))))
  (bind _outactors (Actor|GetAllActorsOfClass "/Game/01_BP/Interactable/BP_SpawnInteractable.BP_SpawnInteractable_C"))
  (bind (_keypin _valuepin) (Utilities|Map|ForEachLoop(Map) _output_get)
    (:then
      (for _index (range 1 _valuepin)
        (bind _returnvalue (Game|SpawnActorfromClass _keypin (Math|Transform|MakeTransform (+ (Math|Vector|MakeVector (Math|Random|RandomFloatinRange -1e+02 1e+02) (Math|Random|RandomFloatinRange -1e+02 1e+02) 0.0) (Transformation|GetActorLocation (.OutItem (Utilities|Array|Random _outactors)))) (Math|Rotator|MakeRotator 0.0 0.0 (Math|Random|RandomFloatinRange 0.0 3.6e+02)) "1.000000,1.000000,1.000000") "Undefined" "MultiplyWithRoot" 0 0 0))
        (Utilities|Array|Add (Variables|Interactable|GetListInteractable) _returnvalue)))))

(event Custom|E_SpawnMovable
  (bind _outactors (Actor|GetAllActorsOfClass "/Game/01_BP/Interactable/BP_SpawnMovable.BP_SpawnMovable_C"))
  (Variables|Movable|SetListSpawnMovable _outactors)
  (switch int (Utilities|Array|Length (Variables|Default|GetListPlayer))
    (:Default
      (bind _output_get (Variables|Movable|SetMapMoverUse (Variables|Movable|GetMapMoverP1) :!label _label)))
    (:1
      (goto _label))
    (:2
      (Variables|Movable|SetMapMoverUse (Variables|Movable|GetMapMoverP2)))
    (:3
      (Variables|Movable|SetMapMoverUse (Variables|Movable|GetMapMoverP3)))
    (:4
      (Variables|Movable|SetMapMoverUse (Variables|Movable|GetMapMoverP4))))
  (bind (_keypin _valuepin) (Utilities|Map|ForEachLoop(Map) _output_get)
    (:then
      (for _index (range 1 _valuepin)
        (bind _returnvalue (Game|SpawnActorfromClass _keypin (Math|Transform|MakeTransform (+ (Math|Vector|MakeVector (Math|Random|RandomFloatinRange -1e+02 1e+02) (Math|Random|RandomFloatinRange -1e+02 1e+02) 0.0) (Transformation|GetActorLocation (.OutItem (Utilities|Array|Random (Variables|Movable|GetListSpawnMovable))))) (Math|Rotator|MakeRotator 0.0 0.0 (Math|Random|RandomFloatinRange 0.0 3.6e+02)) "1.000000,1.000000,1.000000") "Undefined" "MultiplyWithRoot" 0 0 0))
        (Utilities|Array|Add (Variables|Interactable|GetListInteractable) _returnvalue)))))

(event EventBeginPlay
  (bind _asbp_player (Utilities|Casting|CastToBP_Player (Game|Player|GetPlayerPawn 0)))
  (Variables|Default|SetPlayer _asbp_player))

(event EventPostLogin
  (params (NewPlayer :type Player%20Controller%20Object%20Reference)))

(event EventTick
  (params (DeltaSeconds :type Float%20%28single-precision%29))
  (Variables|Default|SetDeltaTime DeltaSeconds)
  (Utilities|FlowControl|Sequence
    (:then_0
      (Development|PrintString (Utilities|String|Append "ActiveFloor : " (Utilities|String|ToString(Integer) (Variables|Default|GetActiveFloor))) true true "(R=0.000000,G=1.000000,B=0.051324,A=1.000000)" 0.0)
      (Development|PrintString (Utilities|String|Append "NB Player :" (Utilities|String|ToString(Integer) (Utilities|Array|Length (Variables|Default|GetListPlayer)))) true true "(R=0.000000,G=1.000000,B=0.051324,A=1.000000)" 0.0)
      (Development|PrintString (Utilities|String|Append "Timer Game : " (Utilities|String|ToString(Float) (Variables|Game|GetTimerGame))) true true "(R=1.000000,G=0.000087,B=0.000000,A=1.000000)" 0.0)
      (for _array_element (Variables|Default|GetListPlayer)
        (Development|PrintString (Utilities|String|Append "Player : " (Utilities|GetDisplayName _array_element)) true true "(R=0.069966,G=1.000000,B=0.000000,A=1.000000)" 0.0)))
    (:then_1
      (CallFunction|FTimer))))

(event EventHandleStartingNewPlayer
  (params (NewPlayer :type Player%20Controller%20Object%20Reference))
  (Utilities|FlowControl|Sequence
    (:then_0
      (bind _returnvalue (Actor|GetActorOfClass "/Script/Engine.PlayerStart"))
      (bind _returnvalue_2 (Game|SpawnActorfromClass "/Game/01_BP/Player/BP_Player.BP_Player_C" (Transformation|GetActorTransform _returnvalue) "AlwaysSpawn" "MultiplyWithRoot" NewPlayer 0))
      (Pawn|Possess NewPlayer _returnvalue_2)
      (Utilities|Array|Add (Variables|Default|GetListPlayer) _returnvalue_2)
      (Default|EActivePlayer _returnvalue_2))))

(event EventOnLogout
  (params (ExitingController :type Controller%20Object%20Reference))
  (for _array_element (Variables|Default|GetListPlayer)
    (if (== (Components|GetOwner _array_element) ExitingController)
      (Utilities|Array|RemoveItem (Variables|Default|GetListPlayer) _array_element))))

(fn ConstructionScript)

(fn FMove
  (params (X :type Float%20%28double-precision%29) (Y :type Float%20%28double-precision%29))
  (Default|FMove (Variables|Default|GetPlayer) X Y))

(fn FDropItem
  (Default|FDropItem (Variables|Default|GetPlayer)))

(fn FRightClick
  (params (Press :type Boolean))
  (Default|FRightClick (Variables|Default|GetPlayer) Press))

(fn FLeftClick
  (params (Press :type Boolean))
  (Default|FLeftClick (Variables|Default|GetPlayer) Press))

(fn FRun
  (params (Press :type Boolean))
  (Default|FRun (Variables|Default|GetPlayer) Press))

(fn FThrowItem
  (Default|FThrowItem (Variables|Default|GetPlayer) 0.0))

(fn SpawnDefaultPawnatTransform
  (params (NewPlayer :type Controller%20Object%20Reference) (SpawnTransform :type Transform%20%28by%20ref%29))
  (return 0))

(fn FChangeLevel
  (params (LevelToLoad :type String))
  (Development|ExecuteConsoleCommand (Utilities|String|Append "ServerTravel " LevelToLoad "?listen") 0))

(fn FStartGame
  (Utilities|FlowControl|Sequence
    (:then_0
      (for _array_element (Variables|Default|GetListeEtage)
        (Variables|/Game/01_BP/Wall/BP_Floor.BP_Floor_C|SetActive _array_element false)
        (Variables|/Game/01_BP/Wall/BP_Floor.BP_Floor_C|SetWaterLevelPercent _array_element 0.0)
        (Variables|/Game/01_BP/Wall/BP_Floor.BP_Floor_C|SetTimerWallBreak _array_element 0.0)
        (Default|FResetAllWall _array_element)))
    (:then_1
      (CallFunction|ESpawnInteractable)
      (CallFunction|ESpawnMovable)
      (for _array_element_2 (Variables|Default|GetListPlayer)
        (Default|EAnimation60s _array_element_2 true)
        (Default|EMoveClient _array_element_2 "-1405.000000,9617.000000,125.000000"))
      (Variables|Game|SetGameStart60s true))))

(fn FTimer
  (if (Variables|Game|GetGameStart60s)
    (bind _output_get (Variables|Game|SetTimerGame (+ (Variables|Game|GetTimerGame) (Variables|Default|GetDeltaTime))))
    (if (> _output_get (- (Variables|Game|GetTimerGamePrepMax) 5.0))
      (Utilities|FlowControl|Sequence
        (:then_0
          (if (not (Variables|Game|GetLaunch60Anim))
            (Variables|Game|SetLaunch60Anim true)
            (for _array_element (Variables|Default|GetListPlayer)
              (Default|EAnimation60s _array_element false)
              (Default|EMoveClient _array_element "-1405.000000,9617.000000,125.000000"))))
        (:then_1
          (if (> _output_get (Variables|Game|GetTimerGamePrepMax))
            (Variables|Game|SetGameStart60s false)
            (Variables|Game|SetGameStart true)
            (Variables|Game|SetTimerGame 0.0)
            (Variables|Game|SetLaunch60Anim false)
            (CallFunction|EActiveFloor 3)
            (goto _label Reset)))))
    (elif (Variables|Game|GetGameStart)
      (bind _output_get_2 (Variables|Game|SetTimerGame (+ (Variables|Game|GetTimerGame) (Variables|Default|GetDeltaTime))))
      (if (> _output_get_2 (Variables|Game|GetTimerGameMax))
        (Utilities|FlowControl|DoOnce false :!label _label
          (:Completed
            (CallFunction|EFinishGame "NewEnumerator1")))))))