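; BP_Floor is one flooding level in a multi-floor game, registered with GM_Gameplay by its Etage index.
; While active, the server updates its walls, breaks random eligible ones on a random timer up to a limit, and raises Water according to the broken count.
; Full water deactivates the floor and activates the next, or finishes the game on the last.
; It also handles wall resets, timeline-driven water changes and per-floor music.
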(event Custom|E_SetWatterTimeline
  (params (AddedWater :type Float%20%28double-precision%29))
  (Timeline|Timeline PlayFromStart
    (:Update
      (Variables|Default|SetWaterLevelPercent (Math|Float|Clamp(Float) (+ (Variables|Default|GetWaterLevelPercent) (* (* (Variables|Default|GetDeltaTime) 2.0) AddedWater)) 0.0 1e+02)))))

(event Custom|E_AddWallBreak
  (params (add :type Boolean))
  (bind _nbwallbreak (Variables|Default|GetNBWallBreak))
  (if add
    (Math|Integer|IncrementInt _nbwallbreak)
    (else
      (Math|Integer|DecrementInt _nbwallbreak))))

(event Custom|E_ActiveFloorClient
  (params (Active :type Boolean))
  (bind _etage (Variables|Default|GetEtage))
  (bind _musicmanager (Variables|Default|GetMusicManager))
  (bind _etage_2 (Variables|Default|GetEtage))
  (bind _output_get (Variables|Default|SetActive Active))
  (if _output_get
    (Utilities|FlowControl|Sequence
      (:then_0
        (Default|ESetAmbiance (Variables|Default|GetMusicManager) _etage_2)
        (if (!= _etage_2 3)
          (if (!= _etage 0)
            (Default|EStartinGameMusic _musicmanager (+ _etage 1) true))
          (else
            (Default|EStartinGameMusic _musicmanager 1 false))))
      (:then_1
        (if (!= (Variables|Default|GetEtage) 0)
          (Default|ELooseFloor (Variables|Default|GetMusicManager)))))))

(event EventTick
  (params (DeltaSeconds :type Float%20%28single-precision%29))
  (Variables|Default|SetDeltaTime DeltaSeconds)
  (if (and (Networking|IsServer) (Variables|Default|GetActive))
    (Utilities|FlowControl|Sequence
      (:then_0
        (for _array_element (Variables|Default|GetListWall)
          (Default|EUpdate _array_element (Variables|Default|GetDeltaTime))))
      (:then_1
        (CallFunction|FCooldownWallBreak)
        (CallFunction|FWaterLevel)
        (Development|PrintString (Utilities|String|Append "NB Wall Brak : " (Utilities|String|ToString(Integer) (Variables|Default|GetNBWallBreak))) true true "(R=0.000000,G=0.660000,B=1.000000,A=1.000000)" 0.0)))))

(event EventBeginPlay
  (if (Networking|IsServer)
    (bind _asgm_gameplay (Utilities|Casting|CastToGM_Gameplay (Game|GetGameMode)))
    (Variables|Default|SetGM _asgm_gameplay)
    (Utilities|Array|SetArrayElem (Variables|/Game/01_BP/GM_Gameplay.GM_Gameplay_C|GetListeEtage (Variables|Default|GetGM)) (Variables|Default|GetEtage) self true)
    (Actor|Tick|SetActorTickEnabled true)
    (Variables|Default|SetTimerBeforeNextWallBreak (Math|Random|RandomFloatinRange 12.0 17.5))
    (for _array_element (Variables|Default|GetListWall)
      (Default|EInit _array_element self))))

(fn ConstructionScript)

(fn FCooldownWallBreak
  (if (< (Variables|Default|GetNbWallBreakNum) (Variables|Default|GetNbWallBreakable))
    (bind _output_get (Variables|Default|SetTimerWallBreak (+ (Variables|Default|GetTimerWallBreak) (Variables|Default|GetDeltaTime))))
    (if (>= _output_get (Variables|Default|GetTimerBeforeNextWallBreak))
      (bind _output_get_2 (LocalVariables|SetF_BreakWall (.OutItem (Utilities|Array|Random (Variables|Default|GetListWall)))))
      (if (Math|Boolean|ORBoolean (Utilities|Enum|Equal(Enum) "NewEnumerator0" (Variables|/Game/01_BP/Wall/BP_Wall.BP_Wall_C|GetState _output_get_2)) (Utilities|Enum|Equal(Enum) (Variables|/Game/01_BP/Wall/BP_Wall.BP_Wall_C|GetState _output_get_2) "NewEnumerator3") (Variables|/Game/01_BP/Wall/BP_Wall.BP_Wall_C|GetOpenable _output_get_2) (Variables|/Game/01_BP/Wall/BP_Wall.BP_Wall_C|GetIsBlocked _output_get_2))
        (Variables|Default|SetTimerBeforeNextWallBreak 0.0)
        (else
          (Variables|Default|SetTimerBeforeNextWallBreak (Math|Random|RandomFloatinRange 12.0 17.5))
          (Variables|Default|SetTimerWallBreak 0.0)
          (Default|EChangeStateClient (LocalVariables|GetF_BreakWall) "NewEnumerator3" 0.0)
          (CallFunction|EAddWallBreak true)
          (Math|Integer|IncrementInt (Variables|Default|GetNbWallBreakNum)
            (:%20%20
              (Development|PrintString "Break Wall"))))))))

(fn FWaterLevel
  (bind _returnvalue (Transformation|GetActorLocation))
  (bind _water (Variables|Default|GetWater))
  (bind _water_2 (Variables|Default|GetWater))
  (bind _gm (Variables|Default|GetGM))
  (bind _etage (Variables|Default|GetEtage))
  (bind _returnvalue_2 (Transformation|GetActorLocation _water_2))
  (bind _returnvalue_3 (Transformation|GetActorLocation _water))
  (bind _output_get (Variables|Default|SetWaterLevelPercent (Math|Float|Clamp(Float) (+ (Variables|Default|GetWaterLevelPercent) (* (Variables|Default|GetNBWallBreak) (* (Variables|Default|GetDeltaTime) 1.0))) 0.0 1e+02)))
  (Transformation|SetActorLocation (Variables|Default|GetWater) (Math|Vector|MakeVector (.x _returnvalue_3) (.y _returnvalue_3) (Math|Float|Lerp (.z _returnvalue) (+ (.z _returnvalue) 2.5e+02) (* (Variables|Default|GetWaterLevelPercent) 0.01))) true false)
  (Development|PrintString (Utilities|String|Append "Water Lvl : " (Utilities|String|ToString(Float) _output_get)) true true "(R=0.000000,G=0.660000,B=1.000000,A=1.000000)" 0.0)
  (if (>= (Variables|Default|GetWaterLevelPercent) 1e+02)
    (Variables|Default|SetActive false)
    (if (< _etage 3)
      (Default|EActiveFloor _gm (+ _etage 1))
      (else
        (Default|EFinishGame _gm "NewEnumerator2")
        (Transformation|SetActorLocation (Variables|Default|GetWater) (Math|Vector|MakeVector (.x _returnvalue_2) (.y _returnvalue_2) 0.0) false true)))))

(fn FResetAllWall
  (Variables|Default|SetNBWallBreak 0)
  (for _array_element (Variables|Default|GetListWall)
    (if (Variables|/Game/01_BP/Wall/BP_Wall.BP_Wall_C|GetOpenable _array_element)
      (Default|ESetRandomBreak _array_element)
      (if (== (Math|Random|RandomIntegerinRange 0 1) 0)
        (Default|EChangeStateClient _array_element "NewEnumerator0" 0.0)
        (CallFunction|EAddWallBreak true)
        (else
          (Default|EChangeStateClient _array_element "NewEnumerator1" 0.0)))
      (else
        (Default|EChangeStateClient _array_element "NewEnumerator1" 0.0)))))