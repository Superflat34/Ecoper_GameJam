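; BP_Window is a wall piece with a window that slides open and closed, extending a parent Blueprint.
; EOpenClose plays or reverses a timeline that moves PivotR vertically to raise or lower it.
; FSetPlancheVisibility extends the parent's state logic: Open and Close show the window and set the window wall mesh and its offset, while Repare and Broken hide the window.
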(event EventEOpenClose
  (params (Open :type Boolean))
  (if Open
    (bind _lerp (Timeline|Timeline Play)
      (:Update
        (Transformation|SetRelativeLocation (Variables|Default|GetPivotR) (Math|Vector|MakeVector 0.0 0.0 (Math|Float|Lerp 0.0 75.0 _lerp)) false false)))
    (else
      (Timeline|Timeline Reverse))))

(fn ConstructionScript
  (|CallParentFunction))

(fn FSetPlancheVisibility
  (bind _window (Variables|Default|GetWindow))
  (bind _wall_straight_2m (Variables|Default|GetWall_Straight_2m))
  (|CallParentFunction)
  (switch Utilities|FlowControl|Switch|SwitchonE_Window (Variables|Default|GetState)
    (:NewEnumerator0
      (Rendering|SetVisibility _window true true :!label _label)
      (Components|StaticMesh|SetStaticMesh _wall_straight_2m "/Game/03_Graph/Meshes/Modules/Walls_Windows/Wall_Window_A_01.Wall_Window_A_01")
      (Transformation|SetRelativeLocation _wall_straight_2m "0.000000,100.000000,0.000000" false true))
    (:NewEnumerator1
      (goto _label))
    (:NewEnumerator2
      (Rendering|SetVisibility _window false true :!label _label_2))
    (:NewEnumerator3
      (goto _label_2))))