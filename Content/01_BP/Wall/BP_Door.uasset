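; BP_Door is a wall piece Blueprint with a door that swings open and closed.
; EOpenClose toggles collision on the door and wall meshes and plays or reverses a timeline, whose update lerps the left pivot's yaw.
; The FSetPlancheVisibility override extends the parent: Open and Close show the Window component and apply the doorway wall mesh and transform, while Repare and Broken hide Window and rotate the wall.
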(event EventEOpenClose
  (params (Open :type Boolean))
  (bind _door (Variables|Default|GetDoor))
  (bind _wall_straight_2m (Variables|Default|GetWall_Straight_2m))
  (if Open
    (Collision|SetCollisionEnabled _door "NoCollision")
    (Collision|SetCollisionEnabled _wall_straight_2m "NoCollision")
    (bind _lerp (Timeline|Timeline_0 Play)
      (:Update
        (Transformation|SetRelativeRotation (Variables|Default|GetPivotL) (Math|Rotator|MakeRotator 0.0 0.0 (Math|Float|Lerp 0.0 1.4e+02 _lerp)) false false)))
    (else
      (Collision|SetCollisionEnabled _door "QueryAndPhysics")
      (Collision|SetCollisionEnabled _wall_straight_2m "QueryAndPhysics")
      (Timeline|Timeline_0 Reverse))))

(fn ConstructionScript
  (|CallParentFunction))

(fn FSetPlancheVisibility
  (bind _window (Variables|Default|GetWindow))
  (bind _wall_straight_2m (Variables|Default|GetWall_Straight_2m))
  (|CallParentFunction)
  (switch Utilities|FlowControl|Switch|SwitchonE_Window (Variables|Default|GetState)
    (:NewEnumerator0
      (Rendering|SetVisibility _window true true :!label _label)
      (Components|StaticMesh|SetStaticMesh _wall_straight_2m "/Game/03_Graph/Meshes/Modules/Wall_StraightDoor_2m_01.Wall_StraightDoor_2m_01")
      (Transformation|SetRelativeLocation _wall_straight_2m "-10.000000,-100.000000,0.000000" false true)
      (Transformation|SetRelativeRotation _wall_straight_2m "0.000000,-270.000000,0.000000" false false))
    (:NewEnumerator1
      (goto _label))
    (:NewEnumerator2
      (Rendering|SetVisibility _window false true :!label _label_2)
      (Transformation|SetRelativeRotation _wall_straight_2m "0.000000,-90.000000,0.000000" false false))
    (:NewEnumerator3
      (goto _label_2))))