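; BP_Wall is a wall belonging to a Floor, with Open, Close, Repare and Broken states, that degrades unless being repaired.
; On the server, closed or repairing walls lose RepareState over time, switching state at thresholds and notifying the Floor when broken.
; State changes set plank visibility or call an empty open/close hook.
; A BP_Movable overlapping its box marks it blocked and updates the Floor's wall-break tracking.
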(event OnComponentBeginOverlap(Box)
  (params (OverlappedComponent :type Primitive%20Component%20Object%20Reference) (OtherActor :type Actor%20Object%20Reference) (OtherComp :type Primitive%20Component%20Object%20Reference) (OtherBodyIndex :type Integer) (bFromSweep :type Boolean) (SweepResult :type Hit%20Result%20Structure%20%28by%20ref%29))
  (if (Networking|IsServer)
    (bind _asbp_movable (Utilities|Casting|CastToBP_Movable OtherActor))
    (Variables|Default|SetObjectBlocked _asbp_movable)
    (Default|EAddWallBreak (Variables|Default|GetFloor) false)
    (Variables|Default|SetIsBlocked true)))

(event OnComponentEndOverlap(Box)
  (params (OverlappedComponent :type Primitive%20Component%20Object%20Reference) (OtherActor :type Actor%20Object%20Reference) (OtherComp :type Primitive%20Component%20Object%20Reference) (OtherBodyIndex :type Integer))
  (if (Networking|IsServer)
    (if (== OtherActor (Variables|Default|GetObjectBlocked))
      (Default|EAddWallBreak (Variables|Default|GetFloor) true)
      (Variables|Default|SetObjectBlocked 0)
      (Variables|Default|SetIsBlocked false))))

(event Custom|E_Update
  (params (DeltaTime :type Float%20%28double-precision%29))
  (Variables|Default|SetDelta%20Time DeltaTime)
  (if (Networking|IsServer)
    (CallFunction|FSubRepareState)))

(event Custom|E_ChangeStateClient
  (params (NewState :type E_Window%20Enum :default "NewEnumerator0") (RepareState :type Float%20%28double-precision%29))
  (bind _output_get (Variables|Default|SetState NewState))
  (switch Utilities|FlowControl|Switch|SwitchonE_Window _output_get
    (:NewEnumerator0
      (CallFunction|EOpenClose true))
    (:NewEnumerator1
      (CallFunction|EOpenClose false))
    (:NewEnumerator2
      (Variables|Default|SetRepareState RepareState :!label _label)
      (CallFunction|FSetPlancheVisibility))
    (:NewEnumerator3
      (goto _label))))

(event Custom|E_Init
  (params (Floor :type BP%20Floor%20Object%20Reference))
  (Variables|Default|SetFloor Floor)
  (Collision|SetCollisionEnabled (Variables|Default|GetBox) "QueryOnly"))

(event Custom|E_OpenClose
  (params (Open :type Boolean)))

(fn ConstructionScript)

(fn FSubRepareState
  (bind _state (Variables|Default|GetState))
  (if (or (Utilities|Enum|Equal(Enum) _state "NewEnumerator1") (Utilities|Enum|Equal(Enum) _state "NewEnumerator2"))
    (if (not (Variables|Default|GetBeingRepared))
      (if (> (Variables|Default|GetRepareState) 5e+01)
        (bind _output_get (Variables|Default|SetRepareState (- (Variables|Default|GetRepareState) (* (Variables|Default|GetDelta%20Time) 4.0))))
        (if (<= _output_get 5e+01)
          (if (not (and (Variables|Default|GetOpenable) (Utilities|Enum|Equal(Enum) (Variables|Default|GetState) "NewEnumerator1")))
            (CallFunction|EChangeStateClient "NewEnumerator2" 5e+01)))
        (else
          (bind _output_get_2 (Variables|Default|SetRepareState (- (Variables|Default|GetRepareState) (* (Variables|Default|GetDelta%20Time) 4.0))))
          (if (<= _output_get_2 0.0)
            (CallFunction|EChangeStateClient "NewEnumerator3" 0.0)
            (Default|EAddWallBreak (Variables|Default|GetFloor) true)))))))

(fn FSetPlancheVisibility
  (bind _planche1 (Variables|Default|GetPlanche1))
  (bind _planche2 (Variables|Default|GetPlanche2))
  (switch Utilities|FlowControl|Switch|SwitchonE_Window (Variables|Default|GetState)
    (:NewEnumerator0
      (Rendering|SetVisibility (Variables|Default|GetPlanche1) false false :!label _label)
      (Rendering|SetVisibility (Variables|Default|GetPlanche2) false false))
    (:NewEnumerator1
      (goto _label))
    (:NewEnumerator2
      (if (> (Variables|Default|GetRepareState) 5e+01)
        (Rendering|SetVisibility _planche1 true false)
        (Rendering|SetVisibility _planche2 true false)
        (else
          (Rendering|SetVisibility _planche1 true false)
          (Rendering|SetVisibility _planche2 false false))))
    (:NewEnumerator3
      (goto _label))))

(fn OnRepCaca)