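; Raft objective that players complete by bringing it planks, a duck and a towel, ending the game once all are in place.
; The server collects overlapping interactables, also counting the duck or towel if either strays too far from the raft.
; Each change passes through a client check event that swaps transparent materials for solid ones to show progress.
; Reset clears progress and respawns the items around random spawn points.
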(event OnComponentBeginOverlap(BoxInteractable)
  (params (OverlappedComponent :type Primitive%20Component%20Object%20Reference) (OtherActor :type Actor%20Object%20Reference) (OtherComp :type Primitive%20Component%20Object%20Reference) (OtherBodyIndex :type Integer) (bFromSweep :type Boolean) (SweepResult :type Hit%20Result%20Structure%20%28by%20ref%29))
  (if (Networking|IsServer)
    (bind _asbp_interactable (Utilities|Casting|CastToBP_Interactable OtherActor))
    (switch Utilities|FlowControl|Switch|SwitchonE_Radeau (Variables|/Game/01_BP/Interactable/BP_Interactable.BP_Interactable_C|GetRadeau _asbp_interactable)
      (:NewEnumerator1
        (Variables|Default|SetHasCanard true))
      (:NewEnumerator2
        (Math|Integer|IncrementInt (Variables|Default|GetNb_Plank)
          (:%20%20
            _)))
      (:NewEnumerator3
        (Variables|Default|SetHasServiette true)))
    (Actor|DestroyActor _asbp_interactable)
    (CallFunction|ECheckCLient (Variables|Default|GetHasServiette) (Variables|Default|GetHasCanard) (Variables|Default|GetNb_Plank))))

(event Custom|E_CheckCLient
  (params (Serviette :type Boolean) (Canard :type Boolean) (Plank :type Integer))
  (Variables|Default|SetHasServiette Serviette)
  (Variables|Default|SetHasCanard Canard)
  (Variables|Default|SetNb_Plank Plank)
  (CallFunction|FCheckRadeau))

(event Custom|E_Reset
  (CallFunction|ECheckCLient false false)
  (CallFunction|FSpawnCanard)
  (CallFunction|FSpawnServiette)
  (CallFunction|FSpawnPlank))

(event EventBeginPlay
  (CallFunction|FCheckRadeau))

(event EventTick
  (params (DeltaSeconds :type Float%20%28single-precision%29))
  (if (Networking|IsServer)
    (Utilities|FlowControl|Sequence
      (:then_0
        (Utilities|IsValid (Variables|Default|GetCanardObject)
          (:Is%20Valid
            (if (> (Math|Vector|Distance(Vector) (Transformation|GetActorLocation (Variables|Default|GetCanardObject)) (Transformation|GetActorLocation)) 1.5e+03)
              (Variables|Default|SetHasCanard true)
              (Actor|DestroyActor (Variables|Default|GetCanardObject))
              (CallFunction|ECheckCLient (Variables|Default|GetHasServiette) (Variables|Default|GetHasCanard) (Variables|Default|GetNb_Plank) :!label _label)))))
      (:then_1
        (Utilities|IsValid (Variables|Default|GetServietteObejct)
          (:Is%20Valid
            (if (> (Math|Vector|Distance(Vector) (Transformation|GetActorLocation (Variables|Default|GetServietteObejct)) (Transformation|GetActorLocation)) 1.5e+03)
              (Variables|Default|SetHasServiette true)
              (Actor|DestroyActor (Variables|Default|GetServietteObejct))
              (goto _label))))))))

(fn ConstructionScript)

(fn FCheckRadeau
  (bind _serviette (Variables|Default|GetServiette))
  (bind _canard (Variables|Default|GetCanard))
  (Utilities|FlowControl|Sequence
    (:then_0
      (for _index (range 0 (- (Variables|Default|GetNb_PlankMax) 1))
        (if (> (Variables|Default|GetNb_Plank) _index)
          (bind _asstatic_mesh_component (Utilities|Casting|CastToStaticMeshComponent (Utilities|Array|Get(acopy) (Components|GetChildrenComponents (Variables|Default|GetPlank) false) _index)))
          (Rendering|Material|SetMaterial _asstatic_mesh_component 0 "/Game/03_Graph/Materials/MI_Plank_01.MI_Plank_01")
          (else
            (bind _asstatic_mesh_component_2 (Utilities|Casting|CastToStaticMeshComponent (Utilities|Array|Get(acopy) (Components|GetChildrenComponents (Variables|Default|GetPlank) false) _index)))
            (Rendering|Material|SetMaterial _asstatic_mesh_component_2 0 "/Game/03_Graph/Materials/FadeRefPlayer/MT_RadeauTransparent.MT_RadeauTransparent")))))
    (:then_1
      (if (Variables|Default|GetHasServiette)
        (Rendering|Material|SetMaterial _serviette 0 "/Game/03_Graph/Materials/MI_Stilts.MI_Stilts")
        (else
          (Rendering|Material|SetMaterial _serviette 0 "/Game/03_Graph/Materials/FadeRefPlayer/MT_RadeauTransparent.MT_RadeauTransparent")))
      (if (Variables|Default|GetHasCanard)
        (Rendering|Material|SetMaterial _canard 0 "/Game/03_Graph/Materials/MI_Duckie.MI_Duckie")
        (else
          (Rendering|Material|SetMaterial _canard 0 "/Game/03_Graph/Materials/FadeRefPlayer/MT_RadeauTransparent.MT_RadeauTransparent"))))
    (:then_2
      (if (Networking|IsServer)
        (if (Math|Boolean|ANDBoolean (>= (Variables|Default|GetNb_Plank) (Variables|Default|GetNb_PlankMax)) (Variables|Default|GetHasCanard) (Variables|Default|GetHasServiette))
          (Default|EFinishGame (Variables|Default|GetGM) "NewEnumerator0"))))))

(fn FSpawnCanard
  (bind _returnvalue (Game|SpawnActorfromClass "/Game/01_BP/Interactable/Movable/BP_Canard.BP_Canard_C" (Math|Transform|MakeTransform (+ (Math|Vector|MakeVector (Math|Random|RandomFloatinRange -5e+01 5e+01) (Math|Random|RandomFloatinRange -5e+01 5e+01) 0.0) (Transformation|GetActorLocation (.OutItem (Utilities|Array|Random (Variables|Default|GetListSpawn))))) (Math|Rotator|MakeRotator 0.0 0.0 (Math|Random|RandomFloatinRange 0.0 3.6e+02)) "1.000000,1.000000,1.000000") "Undefined" "MultiplyWithRoot" 0 0 0))
  (Utilities|Array|Add (Variables|/Game/01_BP/GM_Gameplay.GM_Gameplay_C|GetListInteractable (Variables|Default|GetGM)) _returnvalue)
  (Variables|Default|SetCanardObject _returnvalue))

(fn FSpawnServiette
  (bind _returnvalue (Game|SpawnActorfromClass "/Game/01_BP/Interactable/Movable/BP_Serviette.BP_Serviette_C" (Math|Transform|MakeTransform (+ (Math|Vector|MakeVector (Math|Random|RandomFloatinRange -5e+01 5e+01) (Math|Random|RandomFloatinRange -5e+01 5e+01) 0.0) (Transformation|GetActorLocation (.OutItem (Utilities|Array|Random (Variables|Default|GetListSpawn))))) (Math|Rotator|MakeRotator 0.0 0.0 (Math|Random|RandomFloatinRange 0.0 3.6e+02)) "1.000000,1.000000,1.000000") "Undefined" "MultiplyWithRoot" 0 0 0))
  (Utilities|Array|Add (Variables|/Game/01_BP/GM_Gameplay.GM_Gameplay_C|GetListInteractable (Variables|Default|GetGM)) _returnvalue)
  (Variables|Default|SetServietteObejct _returnvalue))

(fn FSpawnPlank
  (for _index (range 1 (Variables|Default|GetNb_PlankMax))
    (bind _returnvalue (Game|SpawnActorfromClass "/Game/01_BP/Interactable/Interactable/BP_PlankInteractable.BP_PlankInteractable_C" (Math|Transform|MakeTransform (+ (Math|Vector|MakeVector (Math|Random|RandomFloatinRange -5e+01 5e+01) (Math|Random|RandomFloatinRange -5e+01 5e+01) 1e+01) (Transformation|GetActorLocation (.OutItem (Utilities|Array|Random (Variables|Default|GetListSpawn))))) (Math|Rotator|MakeRotator 0.0 0.0 (Math|Random|RandomFloatinRange 0.0 3.6e+02)) "1.000000,1.000000,1.000000") "AlwaysSpawn" "MultiplyWithRoot" 0 0 0))
    (Utilities|Array|Add (Variables|/Game/01_BP/GM_Gameplay.GM_Gameplay_C|GetListInteractable (Variables|Default|GetGM)) _returnvalue)))