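; PC_Player is the player-side input relay, turning Enhanced Input actions into gameplay calls on a GM object.
; FInit stores the GM reference and adds the IMC_Player mapping context to the local player's input subsystem.
; Move, left and right click, run, drop item and throw item events each forward straight to a matching GM function, with no gameplay logic of their own.
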(event Input|EnhancedActionEvents|EnhancedInputActionIA_Move
  (params (ActionValue :type Vector%202D%20Structure) (ElapsedSeconds :type Float%20%28double-precision%29) (TriggeredSeconds :type Float%20%28double-precision%29) (InputAction :type Input%20Action%20Object%20Reference :default "/Game/02_Input/InputAction/IA_Move.IA_Move"))
  (Default|FMove (Variables|Default|GetGM) (.x ActionValue) (.y ActionValue)))

(event Input|EnhancedActionEvents|EnhancedInputActionIA_LeftClick
  (params (ActionValue :type Boolean) (ElapsedSeconds :type Float%20%28double-precision%29) (TriggeredSeconds :type Float%20%28double-precision%29) (InputAction :type Input%20Action%20Object%20Reference :default "/Game/02_Input/InputAction/IA_LeftClick.IA_LeftClick"))
  (Default|FLeftClick (Variables|Default|GetGM) ActionValue))

(event Input|EnhancedActionEvents|EnhancedInputActionIA_RightClick
  (params (ActionValue :type Boolean) (ElapsedSeconds :type Float%20%28double-precision%29) (TriggeredSeconds :type Float%20%28double-precision%29) (InputAction :type Input%20Action%20Object%20Reference :default "/Game/02_Input/InputAction/IA_RightClick.IA_RightClick"))
  (Default|FRightClick (Variables|Default|GetGM) ActionValue))

(event Input|EnhancedActionEvents|EnhancedInputActionIA_DropItem
  (params (ActionValue :type Boolean) (ElapsedSeconds :type Float%20%28double-precision%29) (TriggeredSeconds :type Float%20%28double-precision%29) (InputAction :type Input%20Action%20Object%20Reference :default "/Game/02_Input/InputAction/IA_DropItem.IA_DropItem"))
  (Default|FDropItem (Variables|Default|GetGM)))

(event Input|EnhancedActionEvents|EnhancedInputActionIA_Run
  (params (ActionValue :type Boolean) (ElapsedSeconds :type Float%20%28double-precision%29) (TriggeredSeconds :type Float%20%28double-precision%29) (InputAction :type Input%20Action%20Object%20Reference :default "/Game/02_Input/InputAction/IA_Run.IA_Run"))
  (Default|FRun (Variables|Default|GetGM) ActionValue))

(event Input|EnhancedActionEvents|EnhancedInputActionIA_ThowItem
  (params (ActionValue :type Boolean) (ElapsedSeconds :type Float%20%28double-precision%29) (TriggeredSeconds :type Float%20%28double-precision%29) (InputAction :type Input%20Action%20Object%20Reference :default "/Game/02_Input/InputAction/IA_ThowItem.IA_ThowItem"))
  (Default|FThrowItem (Variables|Default|GetGM)))

(fn ConstructionScript)

(fn FInit
  (params (GM :type GM%20Gameplay%20Object%20Reference))
  (Variables|Default|SetGM GM)
  (Input|AddMappingContext (PlayerController|LocalPlayerSubsystems|GetEnhancedInputLocalPlayerSubsystem (Game|GetPlayerController 0)) "/Game/02_Input/IMC_Player.IMC_Player" 0 (Utilities|Struct|MakeModifyContextOptions true false true)))