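; BP_waterContenant is a usable water container that players fill from a flooded floor and throw out as water.
; When empty, F_Use lowers the active floor's water level through GM_Gameplay, storing the clamped amount if the player stands in water.
; When full, it launches a BP_WaterBall carrying that amount and loses a life, destroying itself at zero.
; E_FilledWaterClient toggles the water visual and plays a random fill or throw sound.
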(event Custom|E_FilledWaterClient
  (params (Filled :type Boolean))
  (bind _audio (Variables|Default|GetAudio))
  (bind _audio_2 (Variables|Default|GetAudio))
  (bind _output_get (Variables|Default|SetIsFilled Filled))
  (Rendering|SetVisibility (Variables|Default|GetWater) _output_get false)
  (if _output_get
    (Audio|Components|Audio|SetSound _audio_2 (.OutItem (Utilities|Array|Random (Variables|Default|GetListSound))))
    (Audio|Components|Audio|Play _audio_2 0.0)
    (else
      (Audio|Components|Audio|SetSound _audio (.OutItem (Utilities|Array|Random (Variables|Default|GetListSoundThrow))))
      (Audio|Components|Audio|Play _audio 0.0))))

(event Custom|E_Destroy
  (Utilities|FlowControl|DelayUntilNextTick)
  (Actor|DestroyActor))

(event EventBeginPlay
  (|CallParentFunction) ; This node is disabled and will not be called.\nDrag off pins to build functionality.
)

(event Collision|EventActorBeginOverlap
  (params (OtherActor :type Actor%20Object%20Reference))
  (|CallParentFunction OtherActor) ; This node is disabled and will not be called.\nDrag off pins to build functionality.
)

(event EventTick
  (params (DeltaSeconds :type Float%20%28single-precision%29))
  (|CallParentFunction DeltaSeconds) ; This node is disabled and will not be called.\nDrag off pins to build functionality.
)

(fn ConstructionScript
  (|CallParentFunction))

(fn FUse
  (params (Player :type BP%20Player%20Object%20Reference))
  (bind _life (Variables|Default|GetLife))
  (if (Variables|Default|GetIsFilled)
    (bind _returnvalue (Game|SpawnActorfromClass "/Game/01_BP/BP_WaterBall.BP_WaterBall_C" (Math|Transform|MakeTransform (Transformation|GetWorldLocation (Variables|/Game/01_BP/Player/BP_Player.BP_Player_C|GetThrowInteractablePos Player)) "0, 0, 0" "1.000000,1.000000,1.000000") "Undefined" "MultiplyWithRoot" 0 (Variables|Default|GetContainWater) 0))
    (Physics|AddForce (Variables|/Game/01_BP/BP_WaterBall.BP_WaterBall_C|GetSphere _returnvalue) (* (+ (Math|Vector|GetForwardVector (Variables|/Script/Engine.Character|GetMesh Player)) "0.000000,0.000000,0.330000") 4e+04) "None" true)
    (Math|Integer|DecrementInt _life
      (:%20%20
        (if (> _life 0)
          (Variables|Default|SetContainWater 0.0)
          (Variables|Default|SetIsFilled false)
          (CallFunction|EFilledWaterClient false)
          (else
            (CallFunction|EDestroy)))))
    (else
      (bind _asgm_gameplay (Utilities|Casting|CastToGM_Gameplay (Game|GetGameMode)))
      (if (and (Variables|/Game/01_BP/Player/BP_Player.BP_Player_C|GetInWater Player) (> (Variables|/Game/01_BP/Wall/BP_Floor.BP_Floor_C|GetWaterLevelPercent (Utilities|Array|Get(acopy) (Variables|/Game/01_BP/GM_Gameplay.GM_Gameplay_C|GetListeEtage _asgm_gameplay) (Variables|/Game/01_BP/GM_Gameplay.GM_Gameplay_C|GetActiveFloor _asgm_gameplay))) 0.0))
        (Default|ESetWatterTimeline (Utilities|Array|Get(acopy) (Variables|/Game/01_BP/GM_Gameplay.GM_Gameplay_C|GetListeEtage _asgm_gameplay) (Variables|/Game/01_BP/GM_Gameplay.GM_Gameplay_C|GetActiveFloor _asgm_gameplay)) (* (Math|Float|Clamp(Float) (Variables|Default|GetSubWater) 0.0 (Variables|/Game/01_BP/Wall/BP_Floor.BP_Floor_C|GetWaterLevelPercent (Utilities|Array|Get(acopy) (Variables|/Game/01_BP/GM_Gameplay.GM_Gameplay_C|GetListeEtage _asgm_gameplay) (Variables|/Game/01_BP/GM_Gameplay.GM_Gameplay_C|GetActiveFloor _asgm_gameplay)))) -1.0))
        (Variables|Default|SetContainWater (Math|Float|Clamp(Float) (Variables|Default|GetSubWater) 0.0 (Variables|/Game/01_BP/Wall/BP_Floor.BP_Floor_C|GetWaterLevelPercent (Utilities|Array|Get(acopy) (Variables|/Game/01_BP/GM_Gameplay.GM_Gameplay_C|GetListeEtage _asgm_gameplay) (Variables|/Game/01_BP/GM_Gameplay.GM_Gameplay_C|GetActiveFloor _asgm_gameplay)))))
        (Variables|Default|SetIsFilled true)
        (CallFunction|EFilledWaterClient true)))))