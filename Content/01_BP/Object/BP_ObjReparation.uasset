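; BP_ObjReparation is a usable, single-use repair object that fixes the wall the player is touching.
; Its FUse function reads the player's WallTouch and changes that wall's state through EChangeStateClient.
; A broken wall becomes half repaired and updates its floor through EAddWallBreak, while a wall repaired halfway or less becomes fully repaired.
; The object destroys itself only when a repair is applied.
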(event EventBeginPlay
  (|CallParentFunction) ; This node is disabled and will not be called.\nDrag off pins to build functionality.
)

(event Collision|EventActorBeginOverlap
  (params (OtherActor :type Actor%20Object%20Reference))
  (|CallParentFunction OtherActor) ; This node is disabled and will not be called.\nDrag off pins to build functionality.
)

(event EventTick
  (params (DeltaSeconds :type Float%20%28single-precision%29))
  (|CallParentFunction DeltaSeconds) ; This node is disabled and will not be called.\nDrag off pins to build functionality.
)

(fn ConstructionScript
  (|CallParentFunction))

(fn FUse
  (params (Player :type BP%20Player%20Object%20Reference))
  (bind _walltouch (Variables|/Game/01_BP/Player/BP_Player.BP_Player_C|GetWallTouch Player))
  (LocalVariables|SetF_Wall _walltouch)
  (Utilities|IsValid _walltouch
    (:Is%20Valid
      (switch Utilities|FlowControl|Switch|SwitchonE_Window (Variables|/Game/01_BP/Wall/BP_Wall.BP_Wall_C|GetState (LocalVariables|GetF_Wall))
        (:NewEnumerator2
          (if (<= (Variables|/Game/01_BP/Wall/BP_Wall.BP_Wall_C|GetRepareState (LocalVariables|GetF_Wall)) 5e+01)
            (Default|EChangeStateClient (LocalVariables|GetF_Wall) "NewEnumerator2" 1e+02)
            (Actor|DestroyActor :!label _label)))
        (:NewEnumerator3
          (Default|EChangeStateClient (LocalVariables|GetF_Wall) "NewEnumerator2" 5e+01)
          (Default|EAddWallBreak (Variables|/Game/01_BP/Wall/BP_Wall.BP_Wall_C|GetFloor (LocalVariables|GetF_Wall)) false)
          (goto _label))))))