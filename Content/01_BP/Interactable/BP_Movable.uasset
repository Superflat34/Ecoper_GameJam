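; Cooperative movable object that several players grab and move together, with walk speed scaled by grabber count against the number required.
; Grabbing attaches the player's PhysicsHandle and constrains their capsule to the mesh through the player's own PhysicsConstraint.
; Four constraint components, picked by grab order, are teleported to grab points and stored on players as move points.
; Releasing undoes the links, zeroes mesh velocities and updates remaining players' speeds.
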(event Custom|E_Grab
  (params (Grab :type Boolean) (Player :type BP%20Player%20Object%20Reference))
  (bind _staticmesh (Variables|Default|GetStaticMesh))
  (bind _listplayergrab (Variables|Default|GetListPlayerGrab))
  (bind _nbplayergrab (Variables|Default|GetNbPlayerGrab))
  (bind _output_get (Variables|/Game/01_BP/Player/BP_Player.BP_Player_C|SetIsGrabbing Player Grab))
  (if _output_get
    (Utilities|Array|Add _listplayergrab Player)
    (CallFunction|FSetPhysicsConstraint true Player)
    (Math|Integer|IncrementInt _nbplayergrab
      (:%20%20
        (CallFunction|EChangePlayerSpeed)
        (Variables|/Game/01_BP/Player/BP_Player.BP_Player_C|SetObjectMove Player self)
        (Class|PhysicsHandleComponent|GrabComponentatLocation (Variables|/Game/01_BP/Player/BP_Player.BP_Player_C|GetPhysicsHandle Player) (Variables|Default|GetStaticMesh) "None" (Transformation|GetWorldLocation (Variables|/Game/01_BP/Player/BP_Player.BP_Player_C|GetThrowInteractablePos Player)))))
    (else
      (CallFunction|FSetPhysicsConstraint false Player)
      (Utilities|Array|RemoveItem _listplayergrab Player)
      (Math|Integer|DecrementInt _nbplayergrab
        (:%20%20
          (CallFunction|EChangePlayerSpeed)
          (Default|FRun Player false)
          (Variables|/Game/01_BP/Player/BP_Player.BP_Player_C|SetObjectMove Player 0)
          (Physics|Components|PhysicsHandle|ReleaseComponent (Variables|/Game/01_BP/Player/BP_Player.BP_Player_C|GetPhysicsHandle Player))
          (Physics|SetPhysicsLinearVelocity _staticmesh "0, 0, 0" false "None")
          (Class|PrimitiveComponent|SetPhysicsAngularVelocityinDegrees _staticmesh "0, 0, 0" false "None"))))))

(event Custom|E_ChangePlayerSpeed
  (for _array_element (Variables|Default|GetListPlayerGrab)
    (Variables|/Script/Engine.CharacterMovementComponent|SetMaxWalkSpeed (Variables|/Script/Engine.Character|GetCharacterMovement _array_element) (* (Variables|Default|GetMaxSpeed) (Math|Float|Clamp(Float) (/ (Variables|Default|GetNbPlayerGrab) (Variables|Default|GetNbPlayerToMove)))))))

(event EventTick
  (params (DeltaSeconds :type Float%20%28single-precision%29))
  (Variables|Default|SetDeltaTime DeltaSeconds))

(fn ConstructionScript
  (|CallParentFunction))

(fn FGuiveObject
  (params (Player :type BP%20Player%20Object%20Reference))
  (LocalVariables|SetF_Player Player)
  (CallFunction|EGrab true (LocalVariables|GetF_Player)))

(fn FSetPhysicsConstraint
  (params (Start :type Boolean) (Player :type BP%20Player%20Object%20Reference))
  (bind _listplayergrabindex (Variables|Default|GetListPlayerGrabIndex))
  (LocalVariables|SetF_Players Player)
  (LocalVariables|SetF_Pos (Transformation|GetWorldLocation (Variables|/Game/01_BP/Player/BP_Player.BP_Player_C|GetGrabMovable (LocalVariables|GetF_Players))))
  (Utilities|FlowControl|Sequence
    (:then_0
      (if Start
        (Utilities|Map|Add _listplayergrabindex (LocalVariables|GetF_Players) (Variables|Default|GetNbPlayerGrab))
        (else
          (Utilities|Map|Remove _listplayergrabindex (LocalVariables|GetF_Players)))))
    (:then_1
      (switch int (.Value (Utilities|Map|Find (Variables|Default|GetListPlayerGrabIndex) (LocalVariables|GetF_Players)))
        (:Default
          (LocalVariables|SetConstraint (Variables|Default|GetPhysicsConstraint) :!label _label))
        (:0
          (goto _label))
        (:1
          (LocalVariables|SetConstraint (Variables|Default|GetPhysicsConstraint1)))
        (:2
          (LocalVariables|SetConstraint (Variables|Default|GetPhysicsConstraint2)))
        (:3
          (LocalVariables|SetConstraint (Variables|Default|GetPhysicsConstraint3))))
      (if Start
        (Transformation|SetWorldLocation (LocalVariables|GetConstraint) (LocalVariables|GetF_Pos) false true)
        (Class|PhysicsConstraintComponent|SetConstrainedComponents (Variables|/Game/01_BP/Player/BP_Player.BP_Player_C|GetPhysicsConstraint (LocalVariables|GetF_Players)) (Variables|/Script/Engine.Character|GetCapsuleComponent (LocalVariables|GetF_Players)) "None" (Variables|Default|GetStaticMesh) "None")
        (Variables|/Game/01_BP/Player/BP_Player.BP_Player_C|SetObjectMovePoint (LocalVariables|GetF_Players) (LocalVariables|GetConstraint))
        (else
          (Variables|/Game/01_BP/Player/BP_Player.BP_Player_C|SetObjectMovePoint (LocalVariables|GetF_Players) 0)
          (Class|PhysicsConstraintComponent|SetConstrainedComponents (Variables|/Game/01_BP/Player/BP_Player.BP_Player_C|GetPhysicsConstraint (LocalVariables|GetF_Players)) (Variables|/Script/Engine.Character|GetCapsuleComponent (LocalVariables|GetF_Players)) "None" (Variables|/Script/Engine.Character|GetCapsuleComponent (LocalVariables|GetF_Players)) "None"))))))