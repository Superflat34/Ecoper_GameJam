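; World pickup for a water item that, when given to a player, becomes an object held in their hand.
; F_GuiveObject spawns the configured class, attaches it to the hand, notifies the client, then destroys the pickup.
; If the spawned item is a BP_waterContenant and HasWater is set, its filled state and water content carry over.
; HasWater is a RepNotify that toggles the Water component's visibility, keeping the look in sync for multiplayer.
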(event EventBeginPlay)

(event Collision|EventActorBeginOverlap
  (params (OtherActor :type Actor%20Object%20Reference)))

(event EventTick
  (params (DeltaSeconds :type Float%20%28single-precision%29)))

(fn ConstructionScript
  (|CallParentFunction))

(fn FGuiveObject
  (params (Player :type BP%20Player%20Object%20Reference))
  (bind _returnvalue (Game|SpawnActorfromClass (Variables|Default|GetObject) (Math|Transform|MakeTransform "0, 0, 0" "0, 0, 0" "1.000000,1.000000,1.000000") "AlwaysSpawn" "MultiplyWithRoot" Player 0))
  (Transformation|AttachComponentToComponent _returnvalue (Variables|/Game/01_BP/Player/BP_Player.BP_Player_C|GetHand Player) "None" "KeepRelative" "KeepRelative" "KeepRelative" true)
  (bind _output_get (Variables|/Game/01_BP/Player/BP_Player.BP_Player_C|SetObjectInHand Player _returnvalue))
  (Default|ESetObjectinHandClient Player _output_get)
  (bind _asbp_water_contenant (Utilities|Casting|CastToBP_waterContenant _returnvalue)
    (:then
      (if (Variables|Default|GetHasWater)
        (Variables|/Game/01_BP/Object/BP_waterContenant.BP_waterContenant_C|SetIsFilled _asbp_water_contenant true)
        (Default|EFilledWaterClient _asbp_water_contenant true)
        (Variables|/Game/01_BP/Object/BP_waterContenant.BP_waterContenant_C|SetContainWater _asbp_water_contenant (Variables|Default|GetWaterInIt))))
    (:CastFailed
      _))
  (Actor|DestroyActor))

(fn OnRepHasWater
  (Rendering|SetVisibility (Variables|Default|GetWater) (Variables|Default|GetHasWater) false))